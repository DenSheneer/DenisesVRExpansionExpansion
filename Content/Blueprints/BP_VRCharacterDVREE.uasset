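; VR character Blueprint that manages posed grasping hands and relays controller drop events through an OnDrop call.
; Gripping calls SetPose, which can refuse to replace a current pose, otherwise respawns that hand and applies or clears its custom animation.
; RespawnHand replaces the GraspingHandManny actor on authority, attaches it to the controller and hides the default hand mesh and grab sphere.
; Hands use physics only when an animation is supplied.
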(event Custom|OnRightDropped
  (params (GripInformation :type BP%20Actor%20Grip%20Information%20Structure%20%28by%20ref%29) (bWasSocketed :type Boolean))
  (Default|CallOnDrop self "Right"))

(event Custom|SetAnimParameter
  (params (Hand :type Grasping%20Hand%20Manny%20Object%20Reference) (Animation :type Anim%20Sequence%20Object%20Reference))
  (Utilities|IsValid Hand
    (:Is%20Valid
      (Utilities|IsValid Animation
        (:Is%20Valid
          (Variables|/Game/VRE/Core/GraspingHands/GraspingHandManny.GraspingHandManny_C|SetCustomAnimation Hand Animation)
          (Variables|/Game/VRE/Core/GraspingHands/GraspingHandManny.GraspingHandManny_C|SetHandAnimState Hand "NewEnumerator3")
          (Variables|/Game/VRE/Core/GraspingHands/GraspingHandManny.GraspingHandManny_C|SetCustomAnimIsSnapShot Hand false)
          (Variables|/Game/VRE/Core/GraspingHands/GraspingHandManny.GraspingHandManny_C|SetHasCustomAnimation Hand true))
        (:Is%20Not%20Valid
          (Variables|/Game/VRE/Core/GraspingHands/GraspingHandManny.GraspingHandManny_C|SetCustomAnimation Hand 0)
          (Variables|/Game/VRE/Core/GraspingHands/GraspingHandManny.GraspingHandManny_C|SetHandAnimState Hand "NewEnumerator1")
          (Variables|/Game/VRE/Core/GraspingHands/GraspingHandManny.GraspingHandManny_C|SetHasCustomAnimation Hand false))))
    (:Is%20Not%20Valid
      (Development|PrintString "no  anim played"))))

(event Custom|OnLeftDropped
  (params (GripInformation :type BP%20Actor%20Grip%20Information%20Structure%20%28by%20ref%29) (bWasSocketed :type Boolean))
  (Default|CallOnDrop self "Left"))

(event Custom|OnLeftGripped
  (params (GripInformation :type BP%20Actor%20Grip%20Information%20Structure%20%28by%20ref%29))
  (CallFunction|SetPose 0 "Left" false))

(event Custom|OnRightGrabbed
  (params (GripInformation :type BP%20Actor%20Grip%20Information%20Structure%20%28by%20ref%29))
  (CallFunction|SetPose 0 "Right" false))

(event EventBeginPlay
  (|CallParentFunction)
  (EventDispatchers|BindEventtoOnDroppedObject (Variables|Default|GetLeftMotionController) (delegate Custom|OnLeftDropped))
  (EventDispatchers|BindEventtoOnDroppedObject (Variables|Default|GetRightMotionController) (delegate Custom|OnRightDropped))
  (EventDispatchers|BindEventtoOnGrippedObject (Variables|Default|GetLeftMotionController) (delegate Custom|OnLeftGripped))
  (EventDispatchers|BindEventtoOnGrippedObject (Variables|Default|GetRightMotionController) (delegate Custom|OnRightGrabbed)))

(fn ConstructionScript
  (|CallParentFunction))

(fn RespawnHand
  (params (HandSide :type EControllerHand%20Enum :default "Left") (UsePhysicalHands :type Boolean) (UseFingerCurls :type Boolean))
  (bind _self self)
  (Utilities|FlowControl|Sequence
    (:then_0
      (switch Utilities|FlowControl|Switch|SwitchonEControllerHand HandSide
        (:Left
          (LocalVariables|SetthisMotionController (Variables|Default|GetLeftMotionController))
          (LocalVariables|SetotherMotionController (Variables|Default|GetRightMotionController))
          (LocalVariables|SetgrabSphere (Variables|Default|GetGrabSphereLeft))
          (LocalVariables|SethandMesh (Variables|Default|GetHandMesh-Left)))
        (:Right
          (LocalVariables|SetthisMotionController (Variables|Default|GetRightMotionController))
          (LocalVariables|SetotherMotionController (Variables|Default|GetLeftMotionController))
          (LocalVariables|SetgrabSphere (Variables|Default|GetGrabSphereRight))
          (LocalVariables|SethandMesh (Variables|Default|GetHandMesh-Right)))))
    (:then_1
      (Networking|SwitchHasAuthority
        (:Authority
          (Utilities|FlowControl|Sequence
            (:then_0
              ;[1 1 1] Clear the grasping hands so we can re-init them
              (switch Utilities|FlowControl|Switch|SwitchonEControllerHand HandSide
                (:Left
                  (Utilities|IsValid (Variables|Default|GetGraspingHandLeft)
                    (:Is%20Valid
                      (Actor|DestroyActor (Variables|Default|GetGraspingHandLeft))
                      (Networking|SwitchHasAuthority
                        (:Authority
                          (Variables|Default|SetGraspingHandLeft 0))
                        (:Remote
                          _))
                      (Development|SetHiddeninGame (Variables|Default|GetHandMesh-Left) false false))
                    (:Is%20Not%20Valid
                      _)))
                (:Right
                  (Utilities|IsValid (Variables|Default|GetGraspingHandRight)
                    (:Is%20Valid
                      (Actor|DestroyActor (Variables|Default|GetGraspingHandRight))
                      (Networking|SwitchHasAuthority
                        (:Authority
                          (Variables|Default|SetGraspingHandRight 0))
                        (:Remote
                          _))
                      (Development|SetHiddeninGame (Variables|Default|GetHandMesh-Right) false false))
                    (:Is%20Not%20Valid
                      _))))
              (CallFunction|SetGripComponents (Variables|Default|GetGrabSphereLeft) (Variables|Default|GetGrabSphereRight)))
            (:then_1
              (bind _returnvalue (Game|SpawnActorfromClass "/Game/VRE/Core/GraspingHands/GraspingHandManny.GraspingHandManny_C" (Transformation|GetWorldTransform (LocalVariables|GethandMesh)) "Undefined" "MultiplyWithRoot" _self (LocalVariables|GetthisMotionController) (select UsePhysicalHands (LocalVariables|GetgrabSphere) 0) (LocalVariables|GetotherMotionController) UseFingerCurls _self))
              (switch Utilities|FlowControl|Switch|SwitchonEControllerHand (Class|GripMotionControllerComponent|GetHandType (LocalVariables|GetthisMotionController))
                (:Left
                  (Variables|Default|SetGraspingHandLeft _returnvalue))
                (:Right
                  (Variables|Default|SetGraspingHandRight _returnvalue)))
              (Transformation|AttachComponentToComponent _returnvalue (LocalVariables|GetthisMotionController) "None" "KeepWorld" "KeepWorld" "KeepWorld" false) ; When welded, cannot use phsysical hands
              (Development|SetHiddeninGame (LocalVariables|GetgrabSphere) true false)
              (return))))
        (:Remote
          (Development|SetHiddeninGame (LocalVariables|GetgrabSphere) true false))))))

(fn SetPose
  (params (Animation :type Anim%20Sequence%20Object%20Reference) (HandSide :type EControllerHand%20Enum :default "Left") (OverrideCurrentPose :type Boolean))
  (Utilities|FlowControl|Sequence
    (:then_0
      (switch Utilities|FlowControl|Switch|SwitchonEControllerHand HandSide
        (:Left
          (bind _graspinghandleft (Variables|Default|GetGraspingHandLeft)
            (:then
              (if (and (not OverrideCurrentPose) (Utilities|Enum|Equal(Enum) (Variables|/Game/VRE/Core/GraspingHands/GraspingHandManny.GraspingHandManny_C|GetHandAnimState _graspinghandleft) "NewEnumerator2"))
                (return false)))
            (:else
              (return false))))
        (:Right
          (bind _graspinghandright (Variables|Default|GetGraspingHandRight)
            (:then
              (if (and (not OverrideCurrentPose) (Utilities|Enum|Equal(Enum) (Variables|/Game/VRE/Core/GraspingHands/GraspingHandManny.GraspingHandManny_C|GetHandAnimState _graspinghandright) "NewEnumerator2"))
                (return false)))
            (:else
              (return false))))))
    (:then_1
      (CallFunction|RespawnHand HandSide (Utilities|IsValid Animation) false)
      (CallFunction|SetGripComponents (Variables|Default|GetGrabSphereLeft) (Variables|Default|GetGrabSphereRight)) ; Choose the gripping components
    )
    (:then_2
      (switch Utilities|FlowControl|Switch|SwitchonEControllerHand HandSide
        (:Left
          (CallFunction|SetAnimParameter (Variables|Default|GetGraspingHandLeft) Animation))
        (:Right
          (CallFunction|SetAnimParameter (Variables|Default|GetGraspingHandRight) Animation)))
      (return true))))